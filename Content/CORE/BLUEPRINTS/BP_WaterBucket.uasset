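; BP_WaterBucket is an interactable pickup that the player collects by holding interact.
; When HoldCheck passes in IFInteractHold and the character's hands are free, it sets HoldingWaterBucket and HoldingItem on the cached BP_ThirdPersonCharacter, then destroys itself.
; Box overlaps toggle the interaction widget and CharacterInRange, though the live pickup path never checks that flag.
; Tap-interact and drop events are empty.
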(event `self.ReceiveBeginPlay`
  (bind _returnvalue (`GameplayStatics.GetActorOfClass` "/Game/ThirdPerson/Blueprints/BP_ThirdPersonCharacter.BP_ThirdPersonCharacter_C"))
  (set `self.PlayerChracterREF` _returnvalue)
  (set `self.Hold Threshold` 0.25))

(event `/Game/ThirdPerson/Blueprints/Interfaces/BPI_Interact.IF_Interact`)

(event `/Game/ThirdPerson/Blueprints/Interfaces/BPI_Interact.IF_InteractHold`
  (params (`Hold Duration` :type "Float (double-precision)"))
  (bind _success (`self.Hold Check` `Hold Duration`))
  (if _success
    (if (not (`/Game/ThirdPerson/Blueprints/BP_ThirdPersonCharacter.HoldingItem` (`self.PlayerChracterREF`)))
      (set `/Game/ThirdPerson/Blueprints/BP_ThirdPersonCharacter.HoldingWaterBucket?` true (`self.PlayerChracterREF`))
      (set `/Game/ThirdPerson/Blueprints/BP_ThirdPersonCharacter.HoldingItem` true (`self.PlayerChracterREF`))
      (`self.K2_DestroyActor`))))

(event `self.Box.OnComponentBeginOverlap`
  (params (OverlappedComponent :type "PrimitiveComponent Object Reference") (OtherActor :type "Actor Object Reference") (OtherComp :type "PrimitiveComponent Object Reference") (OtherBodyIndex :type Integer) (bFromSweep :type Boolean) (SweepResult :type "HitResult Structure (by ref)"))
  (cast `/Game/ThirdPerson/Blueprints/BP_ThirdPersonCharacter` OtherActor)
  (set `self.CharacterInRange` true)
  (`SceneComponent.SetVisibility` (`self.Interaction_Widget`) true false))

(event `self.Box.OnComponentEndOverlap`
  (params (OverlappedComponent :type "PrimitiveComponent Object Reference") (OtherActor :type "Actor Object Reference") (OtherComp :type "PrimitiveComponent Object Reference") (OtherBodyIndex :type Integer))
  (cast `/Game/ThirdPerson/Blueprints/BP_ThirdPersonCharacter` OtherActor)
  (set `self.CharacterInRange` false)
  (`SceneComponent.SetVisibility` (`self.Interaction_Widget`) false false))

(event `/Game/ThirdPerson/Blueprints/Interfaces/BPI_Interact.IF_DropItem`)

(fn `UserConstructionScript`
  (`parent.UserConstructionScript`))
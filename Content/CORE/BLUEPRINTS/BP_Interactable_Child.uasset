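; Child interactable actor Blueprint that responds to a hold-to-interact input through the IFInteractHold event.
; The event passes the hold duration to HoldCheck and, on success, prints a placeholder message where the success logic would go.
; BeginPlay, overlap and Tick are disabled stubs, and the construction script only calls its parent.
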(event `/Game/ThirdPerson/Blueprints/Interfaces/BPI_Interact.IF_InteractHold`
  (params (`Hold Duration` :type "Float (double-precision)"))
  (bind _success (`self.Hold Check` `Hold Duration`))
  (if _success
    (`KismetSystemLibrary.PrintString` "Hold Success Logic")))

(fn `UserConstructionScript`
  (`parent.UserConstructionScript`))
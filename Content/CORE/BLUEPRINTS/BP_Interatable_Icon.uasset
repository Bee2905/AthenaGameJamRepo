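; BP_Interatable_Icon is an interactable icon actor with Warning, Fix and Spam icons plus a radial progress element.
; On BeginPlay it makes the first available icon visible, checked in that order.
; Every tick it billboards all four elements toward the player camera, using a look-at rotation computed from the Warning icon's location.
; The interact event only prints a placeholder hold-success message, with no progress logic in the graph.
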(event `self.ReceiveBeginPlay`
  (if (`self.Warning?`)
    (`SceneComponent.SetVisibility` (`self.Warning`) true false)
    (elif (`self.Fix?`)
      (`SceneComponent.SetVisibility` (`self.Fix`) true false)
      (elif (`self.Spam?`)
        (`SceneComponent.SetVisibility` (`self.Spam`) true false)))))

(event `/Game/ThirdPerson/Blueprints/Interfaces/BPI_Interact.IF_Interact`
  (if true
    (`KismetSystemLibrary.PrintString` "Hold Success Logic")))

(event `self.ReceiveTick`
  (params (DeltaSeconds :type "Float (single-precision)"))
  ;[1 1 1] Rotates Towards Camera
  (`SceneComponent.K2_SetWorldRotation` (`self.Warning`) (`KismetMathLibrary.FindLookAtRotation` (`SceneComponent.K2_GetComponentLocation` (`self.Warning`)) (`SceneComponent.K2_GetComponentLocation` (`PlayerCameraManager.TransformComponent` (`GameplayStatics.GetPlayerCameraManager` 0)))) false false)
  (`SceneComponent.K2_SetWorldRotation` (`self.Fix`) (`KismetMathLibrary.FindLookAtRotation` (`SceneComponent.K2_GetComponentLocation` (`self.Warning`)) (`SceneComponent.K2_GetComponentLocation` (`PlayerCameraManager.TransformComponent` (`GameplayStatics.GetPlayerCameraManager` 0)))) false false)
  (`SceneComponent.K2_SetWorldRotation` (`self.Spam`) (`KismetMathLibrary.FindLookAtRotation` (`SceneComponent.K2_GetComponentLocation` (`self.Warning`)) (`SceneComponent.K2_GetComponentLocation` (`PlayerCameraManager.TransformComponent` (`GameplayStatics.GetPlayerCameraManager` 0)))) false false)
  (`SceneComponent.K2_SetWorldRotation` (`self.RadialProgress`) (`KismetMathLibrary.FindLookAtRotation` (`SceneComponent.K2_GetComponentLocation` (`self.Warning`)) (`SceneComponent.K2_GetComponentLocation` (`PlayerCameraManager.TransformComponent` (`GameplayStatics.GetPlayerCameraManager` 0)))) false false))

(fn `UserConstructionScript`
  (`parent.UserConstructionScript`))